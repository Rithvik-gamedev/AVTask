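; Gameplay ability for a melee-style attack combo of up to three montages, currently unwired: ActivateAbility is empty and the commit and combo chain is disconnected.
; PlayComboHit plays the montage for the current combo index and ends the ability when it finishes or cancels.
; A brief transition flag keeps interruption by the next hit from ending the ability.
; The disconnected chain buffers attack-input gameplay events and advances the combo on combo-window events.
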(event `Play ComboHit`
  (set `self.bIsTransitioning` true)
  (`AbilityTask_PlayMontageAndWait.CreatePlayMontageAndWaitProxy` "None" (`|GetArrayItem` (`self.ComboMontages`) (- (`self.CurrentComboIndex`) 1)) 1.0 "None"
    (:`then`
      (`KismetSystemLibrary.Delay` 0.1)
      (set `self.bIsTransitioning` false))
    (:`OnCompleted`
      (`self.K2_EndAbility` :!label _label))
    (:`OnBlendOut`
      (goto _label))
    (:`OnInterrupted`
      (if (not (`self.bIsTransitioning`))
        (goto _label)))
    (:`OnCancelled`
      (goto _label))))

(event `self.K2_ActivateAbility`)

(event `self.K2_OnEndAbility`
  (params (bWasCancelled :type Boolean)))